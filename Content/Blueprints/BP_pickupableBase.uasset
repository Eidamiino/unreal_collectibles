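; BP_pickupableBase is a base pickup actor that awards score when collected.
; It spins steadily around its yaw each tick from the rotation recorded at BeginPlay.
; Any actor overlap or an Interact call destroys it and adds ScoreToAdd to Points on BP_ThirdPersonGameMode.
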(event EventBeginPlay
  (Variables|Default|SetInitialZRot (.yaw (Transformation|GetActorRotation))))

(event EventTick
  (params (DeltaSeconds :type Float%20%28single-precision%29))
  (Transformation|SetActorRotation (Math|Rotator|MakeRotator 0.0 0.0 (+ (* (Utilities|Time|GetGameTimeinSeconds) 45.0) (Variables|Default|GetInitialZRot)))))

(event Collision|EventActorBeginOverlap
  (params (OtherActor :type Actor%20Object%20Reference))
  (CallFunction|Interact))

(event EventInteract
  (Actor|DestroyActor)
  (bind _asbp_third_person_game_mode (Utilities|Casting|CastToBP_ThirdPersonGameMode (Game|GetGameMode)))
  (bind _output_get (Variables|/Game/ThirdPerson/Blueprints/BP_ThirdPersonGameMode.BP_ThirdPersonGameMode_C|SetPoints _asbp_third_person_game_mode (+ (stale _output_get) (Variables|Default|GetScoreToAdd)))))

(fn ConstructionScript)