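; BP_finalWall is a wall actor that destroys itself once its pressure plates have been stepped on in the correct order.
; On BeginPlay it binds to the stepped-on event of every plate in its PressurePlates array.
; Each event advances a CurrentOrder counter only if the plate's Order matches it, and out-of-order steps are ignored without resetting progress.
; When the counter equals the number of plates, the wall is destroyed.
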(event Custom|plateSteppedOn
  (params (caller :type Actor%20Object%20Reference) (order :type Integer))
  (bind _currentorder (Variables|Default|GetcurrentOrder))
  (if (== order _currentorder)
    (Math|Integer|IncrementInt _currentorder
      (:%20%20
        (if (== _currentorder (Utilities|Array|Length (Variables|Default|GetpressurePlates)))
          (Actor|DestroyActor))))))

(event EventBeginPlay
  (for _array_element (Variables|Default|GetpressurePlates)
    (EventDispatchers|BindEventtoSteppedon _array_element (delegate Custom|plateSteppedOn))))

(event Collision|EventActorBeginOverlap
  (params (OtherActor :type Actor%20Object%20Reference)))

(event EventTick
  (params (DeltaSeconds :type Float%20%28single-precision%29)))

(fn ConstructionScript)