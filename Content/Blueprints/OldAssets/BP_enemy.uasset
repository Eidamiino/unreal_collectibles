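; Simple enemy that roams the navmesh at random and teleports the player to a fixed location on contact.
; Tick picks a random navigable point in a wide radius around itself whenever idle and sends it to a custom AI MoveTo event.
; An IsMoving flag blocks new requests until the move succeeds or fails.
; A Hitbox overlap with the player character triggers the teleport.
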(event OnComponentBeginOverlap(hitbox)
  (params (OverlappedComponent :type Primitive%20Component%20Object%20Reference) (OtherActor :type Actor%20Object%20Reference) (OtherComp :type Primitive%20Component%20Object%20Reference) (OtherBodyIndex :type Integer) (bFromSweep :type Boolean) (SweepResult :type Hit%20Result%20Structure%20%28by%20ref%29))
  (bind _returnvalue (Game|GetPlayerCharacter 0))
  (if (== OtherActor _returnvalue)
    (Transformation|Teleport _returnvalue "900.000000,-2690.000000,1500.000000" "0, 0, 0")))

(event Custom|goToPlace
  (params (location :type Vector))
  (AI|AIMoveTo self location 0 5.0 false
    (:then
      (Variables|Default|SetisMoving true))
    (:OnSuccess
      (Variables|Default|SetisMoving false :!label _label))
    (:OnFail
      (goto _label))))

(event EventBeginPlay)

(event Collision|EventActorBeginOverlap
  (params (OtherActor :type Actor%20Object%20Reference)))

(event EventTick
  (params (DeltaSeconds :type Float%20%28single-precision%29))
  (if (not (Variables|Default|GetisMoving))
    (bind _randomlocation (Class|NavigationSystemV1|GetRandomLocationinNavigableRadius (Transformation|GetActorLocation) 3e+03 0 0))
    (CallFunction|GotoPlace _randomlocation)))

(fn ConstructionScript)