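; BP_goldenSkull is an interactable golden skull that unlocks a door when the player interacts with it.
; On Interact it runs the parent's interaction, destroys the actor held in DoorReference, then sets DoorUnlocked on the player's BP_ThirdPersonCharacter.
; BeginPlay, overlap and Tick are disabled stubs, and the construction script only calls the parent.
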(event EventBeginPlay
  (|CallParentFunction) ; This node is disabled and will not be called.\nDrag off pins to build functionality.
)

(event Collision|EventActorBeginOverlap
  (params (OtherActor :type Actor%20Object%20Reference)))

(event EventTick
  (params (DeltaSeconds :type Float%20%28single-precision%29))
  (|CallParentFunction DeltaSeconds) ; This node is disabled and will not be called.\nDrag off pins to build functionality.
)

(event EventInteract
  (|CallParentFunction)
  (Actor|DestroyActor (Variables|Default|GetdoorReference))
  (bind _asbp_third_person_character (Utilities|Casting|CastToBP_ThirdPersonCharacter (Game|GetPlayerCharacter 0)))
  (Variables|/Game/ThirdPerson/Blueprints/BP_ThirdPersonCharacter.BP_ThirdPersonCharacter_C|SetdoorUnlocked _asbp_third_person_character true))

(fn ConstructionScript
  (|CallParentFunction))