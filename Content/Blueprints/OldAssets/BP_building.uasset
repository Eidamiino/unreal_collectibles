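; Building-placement Blueprint that previews a placeable item where the player aims and spawns the placed copy.
; previewLoop traces from the third-person follow camera and, on a hit, destroys and respawns a BP_placable preview there.
; placeObject spawns the preview's class at that location, blocking Pawn and a custom trace channel.
; Separate events set the yaw, item mesh and index passed to both spawns.
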(event Custom|previewLoop
  (bind _asbp_third_person_character (Utilities|Casting|CastToBP_ThirdPersonCharacter (Game|GetPlayerCharacter 0)))
  (bind (_outhit _returnvalue) (Collision|LineTraceByChannel (.location (Transformation|GetWorldTransform (Variables|/Game/ThirdPerson/Blueprints/BP_ThirdPersonCharacter.BP_ThirdPersonCharacter_C|GetFollowCamera _asbp_third_person_character))) (+ (.location (Transformation|GetWorldTransform (Variables|/Game/ThirdPerson/Blueprints/BP_ThirdPersonCharacter.BP_ThirdPersonCharacter_C|GetFollowCamera _asbp_third_person_character))) (* (Math|Vector|GetForwardVector (.rotation (Transformation|GetWorldTransform (Variables|/Game/ThirdPerson/Blueprints/BP_ThirdPersonCharacter.BP_ThirdPersonCharacter_C|GetFollowCamera _asbp_third_person_character)))) 7e+02)) "TraceTypeQuery1" false 0 "None"))
  (if _returnvalue
    (bind _output_get (Variables|Default|Setlocation (.Location (Collision|BreakHitResult _outhit))))
    (Utilities|IsValid (Variables|Default|GetplacedObject)
      (:Is%20Valid
        (Actor|DestroyActor (Variables|Default|GetplacedObject)))
      (:Is%20Not%20Valid
        _))
    (bind _returnvalue_2 (Game|SpawnActorfromClass "/Game/Blueprints/OldAssets/BP_placable.BP_placable_C" (Math|Transform|MakeTransform _output_get (Math|Rotator|MakeRotator 0.0 0.0 (Variables|Default|GetAmount)) "1.000000,1.000000,1.000000") "Undefined" "MultiplyWithRoot" 0 (Variables|Default|GetIndex) (Variables|Default|GetItem%20Mesh) 0))
    (Variables|Default|SetplacedObject _returnvalue_2)))

(event Custom|placeObject
  (bind _returnvalue (Game|SpawnActorfromClass (Utilities|GetClass (Variables|Default|GetplacedObject)) (Math|Transform|MakeTransform (Variables|Default|Getlocation) (Math|Rotator|MakeRotator 0.0 0.0 (Variables|Default|GetAmount)) "1.000000,1.000000,1.000000") "Undefined" "MultiplyWithRoot" 0 (Variables|Default|GetIndex) (Variables|Default|GetItem%20Mesh) 0))
  (Collision|SetCollisionResponsetoChannel (Variables|/Game/Blueprints/OldAssets/BP_placable.BP_placable_C|Getr _returnvalue) "ECC_Pawn" "ECR_Block")
  (Collision|SetCollisionResponsetoChannel (Variables|/Game/Blueprints/OldAssets/BP_placable.BP_placable_C|Getr _returnvalue) "ECC_GameTraceChannel2" "ECR_Block"))

(event Custom|rotate
  (params (amount :type Float%20%28double-precision%29))
  (bind _output_get (Variables|Default|SetAmount (+ (stale _output_get) amount))))

(event Custom|addIndex
  (params (amount :type Integer))
  (Variables|Default|SetIndex amount))

(event Custom|setItemMesh
  (params (Item%20Mesh :type Static%20Mesh%20Object%20Reference))
  (Variables|Default|SetItem%20Mesh Item%20Mesh))

(event EventBeginPlay)

(event EventTick
  (params (DeltaSeconds :type Float%20%28single-precision%29)))