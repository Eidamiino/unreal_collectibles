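; Base interactable pickup actor that awards score to the player when interacted with.
; Its Interact event destroys the actor and adds its ScoreToAdd value to the Points total stored on BP_ThirdPersonGameMode.
; The new total prints to screen, and a Czech win message follows once it reaches a hard-coded threshold, so the win check lives in the pickup itself.
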(event EventInteract
  (Actor|DestroyActor)
  (bind _asbp_third_person_game_mode (Utilities|Casting|CastToBP_ThirdPersonGameMode (Game|GetGameMode)))
  (bind _output_get (Variables|/Game/ThirdPerson/Blueprints/BP_ThirdPersonGameMode.BP_ThirdPersonGameMode_C|SetPoints _asbp_third_person_game_mode (+ (stale _output_get) (Variables|Default|GetScoreToAdd))))
  (Development|PrintString (Utilities|String|ToString(Integer) _output_get))
  (if (>= _output_get 5)
    (Development|PrintString "VYHRAL JSI")))

(fn ConstructionScript)