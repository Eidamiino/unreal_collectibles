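; BP_npcWalker is an AI-perceiving NPC that reacts to seeing the player.
; On target perception updates, it filters for the sight sense and the player pawn, then raises its walk speed.
; It writes the player to the targetActor Blackboard key, clearing it when sight is lost, and stores the stimulus location as lastKnownLocation.
; The speed boost applies on both gaining and losing sight and is never reset here.
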(event OnPerceptionUpdated(AIPerception)
  (params (UpdatedActors :type Array%20of%20Actor%20Object%20References)))

(event OnTargetPerceptionUpdated(AIPerception)
  (params (Actor :type Actor%20Object%20Reference) (Stimulus :type AI%20Stimulus%20Structure))
  (bind (_age _expirationage _strength _stimuluslocation _receiverlocation _tag _bsuccessfullysensed) (Utilities|Struct|BreakAIStimulus Stimulus))
  (bind _returnvalue (AI|GetBlackboard 0))
  (bind _returnvalue_2 (Class|AIPerceptionSystem|GetSenseClassforStimulus Stimulus))
  (if (== _returnvalue_2 "/Script/AIModule.AISense_Sight")
    (if (== Actor (Game|Player|GetPlayerPawn 0))
      (Variables|/Script/Engine.CharacterMovementComponent|SetMaxWalkSpeed (Variables|Character|GetCharacterMovement) 8e+02)
      (AI|Components|Blackboard|SetValueasObject _returnvalue (Utilities|Name|MakeLiteralName "targetActor") (Utilities|SelectObject (Game|Player|GetPlayerPawn 0) 0 _bsuccessfullysensed))
      (AI|Components|Blackboard|SetValueasVector _returnvalue (Utilities|Name|MakeLiteralName "lastKnownLocation") _stimuluslocation))))

(event EventBeginPlay)

(event Collision|EventActorBeginOverlap
  (params (OtherActor :type Actor%20Object%20Reference)))

(event EventTick
  (params (DeltaSeconds :type Float%20%28single-precision%29)))

(fn ConstructionScript)